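; TrackSegment is a 2D side-scroller track piece with death areas and triggers that extend the track.
; BoxComponents tagged DeathArea call OnDeath on an overlapping side-scroller character.
; Left and right triggers each call Parent.GenerateNext once, only when matching Parent.IsGoingRight, with the construction script pre-locking the opposite side.
; GetTrackLength derives segment length from the bottom floor's X scale.
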(event OnComponentBeginOverlap(GenerateNext_L)
  (params (OtherActor :type Actor%20Object%20Reference) (OtherComp :type Primitive%20Component%20Object%20Reference) (OtherBodyIndex :type Integer) (bFromSweep :type Boolean) (SweepResult :type Hit%20Result%20Structure%20%28by%20ref%29))
  (bind _parent (Variables|Default|GetParent))
  (if (and (not (Variables|/Game/Blueprints/TrackGenerator.TrackGenerator_C|GetIsGoingRight _parent)) (not (Variables|Default|GetHasGen_L)))
    (Variables|Default|SetHasGen_L true)
    (Default|GenerateNext _parent)
    (Development|PrintString "GEN_L")))

(event OnComponentBeginOverlap(GenerateNext_R)
  (params (OtherActor :type Actor%20Object%20Reference) (OtherComp :type Primitive%20Component%20Object%20Reference) (OtherBodyIndex :type Integer) (bFromSweep :type Boolean) (SweepResult :type Hit%20Result%20Structure%20%28by%20ref%29))
  (bind _parent (Variables|Default|GetParent))
  (if (and (Variables|/Game/Blueprints/TrackGenerator.TrackGenerator_C|GetIsGoingRight _parent) (not (Variables|Default|GetHasGen_R)))
    (Variables|Default|SetHasGen_R true)
    (Default|GenerateNext _parent)
    (Development|PrintString (Utilities|GetDisplayName self))))

(event Custom|On%20Death%20Overlap
  (params (OtherActor :type Actor%20Object%20Reference) (OtherComp :type Primitive%20Component%20Object%20Reference) (OtherBodyIndex :type Integer) (bFromSweep :type Boolean) (SweepResult :type Hit%20Result%20Structure%20%28by%20ref%29))
  (bind _as2dside_scroller_character (Utilities|Casting|CastTo2DSideScrollerCharacter OtherActor))
  (Default|OnDeath _as2dside_scroller_character))

(event EventBeginPlay
  (Collision|BindEventtoOnComponentBeginOverlap (Actor|GetComponentsbyTag "/Script/Engine.BoxComponent" "DeathArea") (delegate Custom|On%20Death%20Overlap)))

(event EventActorBeginOverlap
  (params (OtherActor :type Actor%20Object%20Reference)))

(event EventTick
  (params (DeltaSeconds :type Float%20%28single-precision%29)))

(fn ConstructionScript
  (bind _goingright (CallFunction|ShouldGenerateRight))
  (Variables|Default|SetHasGen_R (not _goingright))
  (Variables|Default|SetHasGen_L _goingright))

(fn GetTrackLength
  (return (* (.X (Math|Vector|BreakVector (Transformation|GetWorldScale (Variables|Default|GetBottom%20Floor)))) 5e+01)))

(fn ShouldGenerateRight
  (return (Variables|/Game/Blueprints/TrackGenerator.TrackGenerator_C|GetIsGoingRight (Variables|Default|GetParent))))