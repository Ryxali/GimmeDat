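; Player controller for GimmeDat that drives two local 2D side-scroller characters from a single controller.
; The IsChiefController macro lets only player controller 0 act on movement, jump and slide inputs.
; It forwards the _0 bindings to its own pawn and the _1 bindings to player controller 1's pawn.
; Restart and Quit go to GimmeDatGamemode without that check, with Quit calling RestartGame.
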(event EventBeginPlay)

(event EventTick
  (params (DeltaSeconds :type Float%20%28single-precision%29)))

(event Input|ActionEvents|InputActionJump_0
  (params (Key :type Key%20Structure :default "AnyKey")))

(event Input|ActionEvents|InputActionJump_1
  (params (Key :type Key%20Structure :default "AnyKey")))

(event Input|ActionEvents|InputActionJump_0
  (params (Key :type Key%20Structure :default "AnyKey"))
  (:Pressed
    (Utilities|IsChiefController
      (:Chief
        (bind _as2dside_scroller_character (Utilities|Casting|CastTo2DSideScrollerCharacter (Pawn|GetControlledPawn)))
        (Default|EventInpJump _as2dside_scroller_character)))))

(event Input|ActionEvents|InputActionJump_1
  (params (Key :type Key%20Structure :default "AnyKey"))
  (:Pressed
    (Utilities|IsChiefController
      (:Chief
        (bind _as2dside_scroller_character (Utilities|Casting|CastTo2DSideScrollerCharacter (Pawn|GetControlledPawn (Game|GetPlayerController 1))))
        (Default|EventInpJump _as2dside_scroller_character)))))

(event Input|ActionEvents|InputActionRestart
  (params (Key :type Key%20Structure :default "AnyKey"))
  (:Released
    (bind _asgimme_dat_gamemode (Utilities|Casting|CastToGimmeDatGamemode (Game|GetGameMode)))
    (Default|Restarty _asgimme_dat_gamemode)))

(event Input|ActionEvents|InputActionSlide_0
  (params (Key :type Key%20Structure :default "AnyKey"))
  (:Pressed
    (Utilities|IsChiefController
      (:Chief
        (bind _as2dside_scroller_character (Utilities|Casting|CastTo2DSideScrollerCharacter (Pawn|GetControlledPawn)))
        (Default|InputEvtBeginSlide _as2dside_scroller_character))))
  (:Released
    (Utilities|IsChiefController
      (:Chief
        (bind _as2dside_scroller_character_2 (Utilities|Casting|CastTo2DSideScrollerCharacter (Pawn|GetControlledPawn)))
        (Default|InputEvtEndSlide _as2dside_scroller_character_2)))))

(event Input|ActionEvents|InputActionSlide_1
  (params (Key :type Key%20Structure :default "AnyKey"))
  (:Pressed
    (Utilities|IsChiefController
      (:Chief
        (bind _as2dside_scroller_character (Utilities|Casting|CastTo2DSideScrollerCharacter (Pawn|GetControlledPawn (Game|GetPlayerController 1))))
        (Default|InputEvtBeginSlide _as2dside_scroller_character))))
  (:Released
    (Utilities|IsChiefController
      (:Chief
        (bind _as2dside_scroller_character_2 (Utilities|Casting|CastTo2DSideScrollerCharacter (Pawn|GetControlledPawn (Game|GetPlayerController 1))))
        (Default|InputEvtEndSlide _as2dside_scroller_character_2)))))

(event Input|ActionEvents|InputActionQuit
  (params (Key :type Key%20Structure :default "AnyKey"))
  (:Pressed
    (bind _asgimme_dat_gamemode (Utilities|Casting|CastToGimmeDatGamemode (Game|GetGameMode)))
    (Class|GameMode|RestartGame _asgimme_dat_gamemode)))

(event Input|AxisEvents|InputAxisMoveRight_0
  (params (AxisValue :type Float%20%28single-precision%29))
  (Utilities|IsChiefController
    (:Chief
      (bind _as2dside_scroller_character (Utilities|Casting|CastTo2DSideScrollerCharacter (Pawn|GetControlledPawn)))
      (Default|InputEvtMoveRight _as2dside_scroller_character AxisValue))))

(event Input|AxisEvents|InputAxisMoveRight_1
  (params (AxisValue :type Float%20%28single-precision%29))
  (Utilities|IsChiefController
    (:Chief
      (bind _as2dside_scroller_character (Utilities|Casting|CastTo2DSideScrollerCharacter (Pawn|GetControlledPawn (Game|GetPlayerController 1))))
      (Default|InputEvtMoveRight _as2dside_scroller_character AxisValue))))

(fn ConstructionScript)