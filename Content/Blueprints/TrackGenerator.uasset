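; TrackGenerator is an endless-runner track actor that scrolls three segments along X at the GimmeDatGamemode's current speed.
; Tick moves the trailing segment, snaps the other two to it by track length, and pans a dynamic background material in step with speed.
; GenerateNext destroys the trailing segment, shifts the array and spawns a random segment ahead.
; PerformFlip clears the track, reverses direction and rebuilds the base floor facing the other way.
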(event Custom|PerformFlip
  (params (Callback :type Gimme%20Dat%20Gamemode%20Object%20Reference))
  (CallFunction|Reset)
  (CallFunction|FlipDirection)
  (CallFunction|GenerateBaseFloor))

(event EventBeginPlay
  (CallFunction|GenerateBaseFloor)
  (bind _returnvalue (Rendering|Material|CreateDynamicMaterialInstance (Variables|Default|GetStaticMesh) 0 "/Game/GraphicalAssets/BackgroundMat.BackgroundMat" :!class /Script/Engine.PrimitiveComponent))
  (Variables|Default|SetDynMat _returnvalue))

(event EventActorBeginOverlap
  (params (OtherActor :type Actor%20Object%20Reference)))

(event EventTick
  (params (DeltaSeconds :type Float%20%28single-precision%29))
  (bind _speed (CallFunction|GetGameSpeed))
  (bind _tracks (Variables|Default|GetTracks))
  (bind _tracks_2 (Variables|Default|GetTracks))
  (bind _isgoingright (Variables|Default|GetIsGoingRight))
  (bind _tracks_3 (Variables|Default|GetTracks))
  (bind _item (Utilities|Array|Get(acopy) _tracks_3 2))
  (bind _item_2 (Utilities|Array|Get(acopy) _tracks 2))
  (bind _returnvalue (select _isgoingright -1.0 1.0))
  (bind _asgimme_dat_gamemode (Utilities|Casting|CastToGimmeDatGamemode (Game|GetGameMode)))
  (bind _output_get (Variables|Default|SetPanOffset (+ (Variables|Default|GetPanOffset) (* -0.5 _returnvalue (/ _speed (Variables|/Game/Blueprints/GimmeDatGamemode.GimmeDatGamemode_C|GetMaxGameSpeed _asgimme_dat_gamemode)) DeltaSeconds))))
  (Rendering|Material|SetScalarParameterValue (Variables|Default|GetDynMat) "PanOffset" _output_get :!class /Script/Engine.MaterialInstanceDynamic)
  (if (> (Utilities|Array|Length _tracks_2) 0)
    (Transformation|AddActorWorldOffset (Utilities|Array|Get(acopy) _tracks_2 2) (Math|Vector|MakeVector (* DeltaSeconds _returnvalue _speed) 0.0 0.0))
    (Utilities|FlowControl|Sequence
      (:then_0
        (Transformation|SetActorLocation (Utilities|Array|Get(acopy) (Variables|Default|GetTracks) 1) (+ (Transformation|GetActorLocation _item) (Math|Vector|MakeVector (* 1 (* (Default|GetTrackLength _item) (select (Variables|Default|GetIsGoingRight) 1.0 -1.0) 2.0)) 0.0 0.0)) false false))
      (:then_1
        (Transformation|SetActorLocation (Utilities|Array|Get(acopy) (Variables|Default|GetTracks)) (+ (Transformation|GetActorLocation _item_2) (Math|Vector|MakeVector (* 2 (* (Default|GetTrackLength _item_2) (select (Variables|Default|GetIsGoingRight) 1.0 -1.0) 2.0)) 0.0 0.0)) false false)))))

(event Input|KeyboardEvents|F
  (params (Key :type Key%20Structure :default "AnyKey")))

(fn ConstructionScript)

(fn Reset
  (bind _tracks (Variables|Default|GetTracks))
  (Actor|DestroyActor _tracks)
  (Utilities|Array|Clear _tracks))

(fn GenerateNext
  (bind _tracks (Variables|Default|GetTracks))
  (bind _tracks_2 (Variables|Default|GetTracks))
  (bind _tracks_3 (Variables|Default|GetTracks))
  (Actor|DestroyActor (Utilities|Array|Get(acopy) _tracks_2 2))
  (Utilities|FlowControl|Sequence
    (:then_0
      (Utilities|Array|SetArrayElem _tracks_3 2 (Utilities|Array|Get(acopy) _tracks_3 1)))
    (:then_1
      (Utilities|Array|SetArrayElem _tracks 1 (Utilities|Array|Get(acopy) _tracks))
      (bind _returnvalue (Game|SpawnActorfromClass (CallFunction|GetRandomSegment) (Math|Transform|MakeTransform (+ (Transformation|GetActorLocation (Utilities|Array|Get(acopy) _tracks_2 1)) (* (select (Variables|Default|GetIsGoingRight) "1.000000,0.000000,0.000000" "-1.000000,0.000000,0.000000") 6e+03)) (Math|Vector|RotatorfromAxisandAngle "0, 0,1.000000" (select (Variables|Default|GetIsGoingRight) 1.8e+02 0.0))) "Undefined" 0 self 0))
      (Utilities|Array|SetArrayElem (Variables|Default|GetTracks) 0 _returnvalue))))

(fn FlipDirection
  (Variables|Default|SetIsGoingRight (not (Variables|Default|GetIsGoingRight))))

(fn GenerateBaseFloor
  (for _index (range -1 1)
    (bind _returnvalue (Game|SpawnActorfromClass "/Game/Blueprints/TrackSegment.TrackSegment_C" (Math|Transform|MakeTransform (Math|Vector|MakeVector (* _index (select (Variables|Default|GetIsGoingRight) -6e+03 6e+03)) 0.0 (.Z (Math|Vector|BreakVector (Transformation|GetActorLocation)))) (Math|Vector|RotatorfromAxisandAngle "0, 0,1.000000" (select (Variables|Default|GetIsGoingRight) 1.8e+02 0.0))) "AlwaysSpawn" 0 self 0))
    (Utilities|Array|Add (Variables|Default|GetTracks) _returnvalue)))

(fn GetRandomSegment
  (bind _tracksegments (Variables|Default|GetTrackSegments))
  (return (Utilities|Array|Get(acopy) _tracksegments (Math|Random|RandomIntegerinRange 0 (- (Utilities|Array|Length _tracksegments) 1)))))

(fn GetGameSpeed
  (bind _asgimme_dat_gamemode (Utilities|Casting|CastToGimmeDatGamemode (Game|GetGameMode))
    (:then
      (return (Variables|/Game/Blueprints/GimmeDatGamemode.GimmeDatGamemode_C|GetCurrentGameSpeed _asgimme_dat_gamemode)))
    (:CastFailed
      (return 0.0))))