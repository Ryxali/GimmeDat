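; GimmeDatGameInstance is the game instance that manages the main menu and the start of a match.
; ShowMainMenu creates the MainMenu widget, stores it, adds it to the viewport and shows the mouse cursor.
; StartGame calls StartMatch on GimmeDatGamemode, then HideMainMenu removes the widget, hides the cursor and returns focus to the game viewport.
; The Init event is empty, so nothing in this asset opens the menu automatically.
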(event EventInit)

(fn ShowMainMenu
  (bind _returnvalue (UserInterface|CreateWidget "/Game/Blueprints/MainMenu.MainMenu_C"))
  (bind _output_get (Variables|Default|SetMenuWidget _returnvalue))
  (UserInterface|Viewport|AddtoViewport _output_get 10)
  (Variables|/Script/Engine.PlayerController|SetbShowMouseCursor (Game|GetPlayerController 0) true))

(fn HideMainMenu
  (Widget|RemovefromParent (Variables|Default|GetMenuWidget))
  (Variables|/Script/Engine.PlayerController|SetbShowMouseCursor (Game|GetPlayerController 0) false)
  (Class|WidgetBlueprintLibrary|SetFocustoGameViewport))

(fn StartGame
  (bind _asgimme_dat_gamemode (Utilities|Casting|CastToGimmeDatGamemode (Game|GetGameMode)))
  (Class|GameMode|StartMatch _asgimme_dat_gamemode)
  (CallFunction|HideMainMenu))