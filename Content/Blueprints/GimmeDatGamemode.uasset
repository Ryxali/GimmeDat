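; Game mode for a local two-player chase side-scroller, Purple versus Green, with a game speed that ramps up to a cap.
; Match start spawns both colored players, the track and DatItem; BeginPlay creates player two, the tracking camera and menu.
; Deaths trigger DatItem's flip: a dead chased player swaps roles, camera and track, while a dead chaser loses.
; A gate halts the speed ramp after a win until Restarty.
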(event Custom|FlipComplete)

(event Custom|DeathSequenceComplete
  (Utilities|FlowControl|Sequence
    (:then_0
      (Utilities|FlowControl|DoOnce false) ; enters at Reset
    )
    (:then_1
      (Utilities|Time|SetGlobalTimeDilation 1.0)
      (Variables|Default|SetCurrentGameSpeed (Variables|Default|GetStartGameSpeed))
      (if (== (stale Custom|OnPlayerDeath Character) (select (Variables|Default|Getp0_turn) (Game|GetPlayerCharacter 0) (Game|GetPlayerCharacter 1)))
        (bind _output_get (Variables|Default|Setp0_turn (not (Variables|Default|Getp0_turn))))
        (Default|FocusTarget (Variables|Default|GetCameraTarget) (select _output_get (Game|GetPlayerCharacter 0) (Game|GetPlayerCharacter 1)))
        (bind _outactors (Actor|GetAllActorsOfClass "/Game/Blueprints/TrackGenerator.TrackGenerator_C"))
        (Default|PerformFlip _outactors self)
        (bind _asgame_widget (Utilities|Casting|CastToGameWidget (UserInterface|GetUserWidgetObject (Variables|/Game/Blueprints/CameraTracker.CameraTracker_C|GetGameHUDWidget (Variables|Default|GetCameraTarget)))))
        (Default|Annouce _asgame_widget (select (Variables|Default|Getp0_turn) "PURPLE IS BEING CHASED" "GREEN IS BEING CHASED"))
        (Audio|Components|Audio|Play (Variables|Default|GetFlippetyfloppety) 0.0)
        (bind _as2dside_scroller_character (Utilities|Casting|CastTo2DSideScrollerCharacter (Game|GetPlayerCharacter 0)))
        (Default|ResetZ _as2dside_scroller_character)
        (bind _as2dside_scroller_character_2 (Utilities|Casting|CastTo2DSideScrollerCharacter (Game|GetPlayerCharacter 1)))
        (Default|ResetZ _as2dside_scroller_character_2)
        (else
          (Variables|Default|SetCurrentGameSpeed 0.0)
          (bind _outactors_2 (Actor|GetAllActorsOfClass "/Game/Blueprints/TrackGenerator.TrackGenerator_C"))
          (Default|Reset _outactors_2)
          (Default|GenerateBaseFloor _outactors_2)
          (bind _asgame_widget_2 (Utilities|Casting|CastToGameWidget (UserInterface|GetUserWidgetObject (Variables|/Game/Blueprints/CameraTracker.CameraTracker_C|GetGameHUDWidget (Variables|Default|GetCameraTarget)))))
          (Default|ShowWinText _asgame_widget_2 (select (Variables|Default|Getp0_turn) "PURPLE WINS" "GREEN WINS"))
          (Audio|Components|Audio|Play (Variables|Default|GetGameJam_SoundFX_-_TVEndGame) 0.0)
          (Utilities|FlowControl|Sequence
            (:then_0
              (Utilities|FlowControl|Gate false) ; enters at Close
            )
            (:then_1
              (Utilities|FlowControl|DoOnce true) ; enters at Reset
            )))))))

(event Custom|Show%20Game%20Menu)

(event Custom|OnPlayerDeath
  (params (Character :type 2D%20Side%20Scroller%20Character%20Object%20Reference))
  (Utilities|FlowControl|DoOnce false
    (:Completed
      (Default|FLIPFLOP (Variables|Default|GetDatItem) Character))))

(event Custom|Restarty
  (Utilities|FlowControl|DoOnce true
    (:Completed
      (Utilities|FlowControl|Sequence
        (:then_0
          (Utilities|FlowControl|Gate false) ; enters at Open
        )
        (:then_1
          (Variables|Default|SetCurrentGameSpeed (Variables|Default|GetStartGameSpeed))
          (bind _asgame_widget (Utilities|Casting|CastToGameWidget (UserInterface|GetUserWidgetObject (Variables|/Game/Blueprints/CameraTracker.CameraTracker_C|GetGameHUDWidget (Variables|Default|GetCameraTarget)))))
          (Default|HideWinText _asgame_widget))))))

(event EventBeginPlay
  (Variables|Default|SetCurrentGameSpeed (Variables|Default|GetStartGameSpeed))
  (Class|GameplayStatics|CreatePlayer 1)
  (bind _outactors (Actor|GetAllActorsOfClass "/Script/Engine.CameraActor"))
  (Actor|DestroyActor _outactors)
  (bind _returnvalue (Game|SpawnActorfromClass "/Game/Blueprints/CameraTracker.CameraTracker_C" (Math|Transform|MakeTransform "0, 0, 0") "AlwaysSpawn" 0 0))
  (Variables|Default|SetCameraTarget _returnvalue)
  (bind _asgimme_dat_game_instance (Utilities|Casting|CastToGimmeDatGameInstance (Game|GetGameInstance)))
  (Default|ShowMainMenu _asgimme_dat_game_instance)
  (Audio|Components|Audio|Play (Variables|Default|GetMenuMusicLoop) 0.0))

(event EventOnSetMatchState
  (params (NewState :type Name))
  (bind _returnvalue (Game|GetPlayerController 1))
  (bind _returnvalue_2 (Game|GetPlayerController 0))
  (switch name NewState
    (:InProgress
      (Actor|DestroyActor (Game|Player|GetPlayerPawn 0))
      (Actor|DestroyActor (Game|Player|GetPlayerPawn 1))
      (bind _returnvalue_3 (Game|SpawnActorfromClass (Variables|Default|GetDefaultPawnClass) (Math|Transform|MakeTransform "300.000000,0.000000,100.000000" "0.000000, 0, 0") "Undefined" _returnvalue_2 0))
      (Pawn|Possess _returnvalue_2 _returnvalue_3)
      (Utilities|FlowControl|Sequence
        (:then_0
          (Default|FocusTarget (Variables|Default|GetCameraTarget) _returnvalue_3)
          (bind _returnvalue_4 (Game|SpawnActorfromClass (Variables|Default|GetDefaultPawnClass) (Math|Transform|MakeTransform "-300.000000,0.000000,100.000000" "0.000000, 0, 0") "Undefined" _returnvalue 0))
          (Pawn|Possess _returnvalue _returnvalue_4)
          (Utilities|FlowControl|Sequence
            (:then_0
              (Variables|Default|SetCurrentGameSpeed (Variables|Default|GetStartGameSpeed))
              (bind _outactors (Actor|GetAllActorsOfClass "/Game/Blueprints/TrackGenerator.TrackGenerator_C"))
              (Default|Reset _outactors)
              (Default|GenerateBaseFloor _outactors)
              (Audio|Components|Audio|Stop (Variables|Default|GetMenuMusicLoop))
              (Audio|Components|Audio|Play (Variables|Default|GetRunLoop) 0.0)
              (Audio|Components|Audio|Play (Variables|Default|GetGameMusicLoop) 0.0)
              (bind _as2dside_scroller_character (Utilities|Casting|CastTo2DSideScrollerCharacter (Game|GetPlayerCharacter 0)))
              (bind _as2dside_scroller_character_2 (Utilities|Casting|CastTo2DSideScrollerCharacter (Game|GetPlayerCharacter 1)))
              (bind _returnvalue_5 (Game|SpawnActorfromClass "/Game/Blueprints/DatItem.DatItem_C" (Math|Transform|MakeTransform "0, 0, 0") "Undefined" 0 _as2dside_scroller_character _as2dside_scroller_character_2))
              (Variables|Default|SetDatItem _returnvalue_5))
            (:then_1
              (bind _as2dside_scroller_character_3 (Utilities|Casting|CastTo2DSideScrollerCharacter _returnvalue_4))
              (Rendering|Material|SetMaterial (Variables|/Game/2DSideScrollerBP/Blueprints/2DSideScrollerCharacter.2DSideScrollerCharacter_C|GetSkeletalMesh _as2dside_scroller_character_3) 0 "/Game/GraphicalAssets/Mat_Digital_Green.Mat_Digital_Green"))))
        (:then_1
          (bind _as2dside_scroller_character_4 (Utilities|Casting|CastTo2DSideScrollerCharacter _returnvalue_3))
          (Rendering|Material|SetMaterial (Variables|/Game/2DSideScrollerBP/Blueprints/2DSideScrollerCharacter.2DSideScrollerCharacter_C|GetSkeletalMesh _as2dside_scroller_character_4) 0 "/Game/GraphicalAssets/Mat_Digital_Purple.Mat_Digital_Purple"))))))

(event EventTick
  (params (DeltaSeconds :type Float%20%28single-precision%29))
  (Utilities|FlowControl|Gate false
    (:Exit
      (Variables|Default|SetCurrentGameSpeed (Math|Float|Min(Float) (+ (* DeltaSeconds (Variables|Default|GetGameSpeedGainPerSecond)) (Variables|Default|GetCurrentGameSpeed)) (Variables|Default|GetMaxGameSpeed))))))

(event EventInitStartSpot
  (params (StartSpot :type Actor%20Object%20Reference) (NewPlayer :type Controller%20Object%20Reference))
  (Development|PrintString "SPAWNAY"))

(fn ConstructionScript)

(fn OnVolumeChange
  (bind _asgimme_dat_game_instance (Utilities|Casting|CastToGimmeDatGameInstance (Game|GetGameInstance)))
  (for _array_element (Actor|GetComponentsByClass "/Script/Engine.AudioComponent")
    (Audio|Components|Audio|SetVolumeMultiplier _array_element (Variables|/Game/Blueprints/GimmeDatGameInstance.GimmeDatGameInstance_C|GetMusicVolume _asgimme_dat_game_instance) :!class /Script/Engine.AudioComponent)))