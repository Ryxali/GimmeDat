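; DatItem is a carried item in a two-player game that starts in Player0's hand socket and ends up with the survivor after a death.
; FLIP_FLOP runs a timeline that slows global time, offsets the item's own dilation to compensate, and boosts post-process bloom.
; If the holder died, the item detaches and spins across to the other player.
; When finished, it restores effects, attaches to the survivor and notifies GimmeDatGamemode.
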(event Custom|FLIP_FLOP
  (params (Dead%20Guy :type 2D%20Side%20Scroller%20Character%20Object%20Reference) (CamTracker :type Post%20Process%20Volume%20Object%20Reference))
  (bind _settings (Variables|/Script/Engine.PostProcessVolume|GetSettings CamTracker))
  (if (== Dead%20Guy (Variables|Default|GetCurrent))
    (Class|Actor|DetachRootComponentfromParent true))
  (Variables|Default|SetStartBloom (Utilities|Struct|BreakPostProcessSettings _settings))
  (bind (_direction _newtrack_0 _fly_cool _rotatecool _fuckedupgraphx) (Timeline|SlowmoCoolness PlayFromStart)
    (:Update
      (Utilities|FlowControl|Sequence
        (:then_0
          (Utilities|Time|SetGlobalTimeDilation _newtrack_0)
          (Variables|Default|SetCustomTimeDilation (/ 1.0 _newtrack_0)))
        (:then_1
          (if (== Dead%20Guy (Variables|Default|GetCurrent))
            (Transformation|SetActorLocation (Math|Vector|Lerp(Vector) (Transformation|GetActorLocation (Variables|Default|GetCurrent)) (Transformation|GetActorLocation (CallFunction|GetOther)) _fly_cool) false false)
            (Transformation|SetRelativeRotation (Variables|Default|GetScene) (Math|Vector|RotatorfromAxisandAngle "0,1.000000,0.000000" _rotatecool) false false)))
        (:then_2
          (Utilities|Struct|SetmembersinPostProcessSettings _settings (+ _fuckedupgraphx (Variables|Default|GetStartBloom))))))
    (:Finished
      (Utilities|Struct|SetmembersinPostProcessSettings _settings (Variables|Default|GetStartBloom))
      (Variables|Default|SetCurrent (select (== Dead%20Guy (Variables|Default|GetCurrent)) (CallFunction|GetOther) (Variables|Default|GetCurrent)))
      (Transformation|SetRelativeRotation (Variables|Default|GetScene) "0, 0, 0" false false)
      (Utilities|Time|SetGlobalTimeDilation 1.0)
      (Variables|Default|SetCustomTimeDilation 1.0)
      (Class|Actor|AttachRootComponentto (Variables|/Game/2DSideScrollerBP/Blueprints/2DSideScrollerCharacter.2DSideScrollerCharacter_C|GetSkeletalMesh (select (== (Variables|Default|GetPlayer0) Dead%20Guy) (Variables|Default|GetPlayer1) (Variables|Default|GetPlayer0))) "Item_R" "SnapToTarget" true)
      (bind _asgimme_dat_gamemode (Utilities|Casting|CastToGimmeDatGamemode (Game|GetGameMode)))
      (Default|DeathSequenceComplete _asgimme_dat_gamemode))))

(event EventBeginPlay
  (bind _output_get (Variables|Default|SetCurrent (Variables|Default|GetPlayer0)))
  (Class|Actor|AttachRootComponentto (Variables|/Game/2DSideScrollerBP/Blueprints/2DSideScrollerCharacter.2DSideScrollerCharacter_C|GetSkeletalMesh _output_get) "Item_R" "SnapToTarget" true))

(event EventActorBeginOverlap
  (params (OtherActor :type Actor%20Object%20Reference)))

(event EventTick
  (params (DeltaSeconds :type Float%20%28single-precision%29)))

(fn ConstructionScript)

(fn GetOther
  (bind _player0 (Variables|Default|GetPlayer0))
  (return (select (== _player0 (Variables|Default|GetCurrent)) (Variables|Default|GetPlayer1) _player0)))