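; Shared camera actor that both local player controllers view from BeginPlay, following one target player at a time.
; FocusTarget sets that player, and Tick copies its X and Y while holding Z at a fixed height.
; Tick also resizes the HUD and menu widgets to the camera's ortho width and aspect ratio.
; Unconnected nodes, including a two-player midpoint calculation, never run.
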(event EventBeginPlay
  (Game|Player|SetViewTargetwithBlend (Game|GetPlayerController 1) self 0.0 "VTBlend_Linear" 0.0 false))

(event EventActorBeginOverlap
  (params (OtherActor :type Actor%20Object%20Reference)))

(event EventTick
  (params (DeltaSeconds :type Float%20%28single-precision%29))
  (bind _camera (Variables|Default|GetCamera))
  (bind _targetplayer (Variables|Default|GetTargetPlayer))
  (bind _returnvalue (Transformation|GetActorLocation _targetplayer))
  (bind _orthowidth (Variables|/Script/Engine.CameraComponent|GetOrthoWidth _camera))
  (bind (_x _y) (Math|Vector|BreakVector _returnvalue))
  (Class|WidgetComponent|SetDrawSize (Variables|Default|GetGameHUDWidget) (Math|Vector2D|MakeVector2D _orthowidth (/ _orthowidth (Variables|/Script/Engine.CameraComponent|GetAspectRatio _camera))))
  (Utilities|IsValid _targetplayer
    (:Is%20Valid
      (Transformation|SetActorLocation (Math|Vector|MakeVector _x _y 2.5e+02) false false))))

(fn ConstructionScript)

(fn FocusTarget
  (params (Player%20Character :type Actor%20Object%20Reference))
  (Variables|Default|SetTargetPlayer Player%20Character))